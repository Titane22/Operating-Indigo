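; Player controller Blueprint that colors grid tiles to show movement, attack, tracing and path states.
; Its ShowStateOfTile event loops over every Tile_BP actor and sends it to a per-state function that sets tile visibility and its GridMatRef material's color and opacity.
; Movable and attackable highlights, including traced variants, apply only when SelectedCharacter's controller is a PlayerAIController.
; Tracing and path highlights always apply, and stateless tiles are hidden.
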(event `self.ShowStateOfTile`
  ;[1 1 1] Tracing the Grid
  (bind _outactors (`GameplayStatics.GetAllActorsOfClass` "/Game/Blueprints/Tile_BP.Tile_BP_C"))
  (for _array_element _outactors
    (switch `ETileState` (`Tile.GetTileState` _array_element)
      (:`Movable`
        (`self.Movable Material` _array_element))
      (:`Attackable`
        (`self.Attackable Material` _array_element))
      (:`Tracing`
        (`self.Tracing Material` _array_element))
      (:`TracingMovable`
        (`self.Tracing Movable Material` _array_element))
      (:`TracingAttackable`
        (`self.Tracing Attackable Material` _array_element))
      (:`Path`
        (`self.Path Material` _array_element))
      (:`None`
        (`self.None Of State Material` _array_element)))))

(fn `Attackable Material`
  (params (Tile :type "/Game/Blueprints/Tile_BP Object Reference"))
  (bind _gridmat_ref (`/Game/Blueprints/Tile_BP.GridMat_Ref` Tile))
  (bind _returnvalue (`self.CheckPlayerController`))
  (if _returnvalue
    (`SceneComponent.SetVisibility` (`/Game/Blueprints/Tile_BP.Tile` Tile) true false)
    (`MaterialInstanceDynamic.SetVectorParameterValue` _gridmat_ref "BaseColor" (struct :`R` 0.588542 :`G` 0.216704 :`B` 0.061306 :`A` 1.0))
    (`MaterialInstanceDynamic.SetScalarParameterValue` _gridmat_ref "Opacity" 0.5)))

(fn `Check Player Controller`
  (returns (True :type Boolean))
  (cast `PlayerAIController` (`Pawn.GetController` (`self.SelectedCharacter`))
    (:`then`
      (return true))
    (:`CastFailed`
      (return false))))

(fn `Movable Material`
  (params (Tile :type "/Game/Blueprints/Tile_BP Object Reference"))
  (bind _gridmat_ref (`/Game/Blueprints/Tile_BP.GridMat_Ref` Tile))
  (bind _returnvalue (`self.CheckPlayerController`))
  (if _returnvalue
    (`SceneComponent.SetVisibility` (`/Game/Blueprints/Tile_BP.Tile` Tile) true false)
    (`MaterialInstanceDynamic.SetVectorParameterValue` _gridmat_ref "BaseColor" (struct :`R` 0.090238 :`G` 0.692708 :`B` 0.06019 :`A` 1.0))
    (`MaterialInstanceDynamic.SetScalarParameterValue` _gridmat_ref "Opacity" 0.5)))

(fn `None Of State Material`
  (params (Tile :type "/Game/Blueprints/Tile_BP Object Reference"))
  (bind _gridmat_ref (`/Game/Blueprints/Tile_BP.GridMat_Ref` Tile))
  (`SceneComponent.SetVisibility` (`/Game/Blueprints/Tile_BP.Tile` Tile) false false)
  (`MaterialInstanceDynamic.SetVectorParameterValue` _gridmat_ref "BaseColor" (struct :`R` 0.512176 :`G` 0.619792 :`B` 0.506809 :`A` 1.0))
  (`MaterialInstanceDynamic.SetScalarParameterValue` _gridmat_ref "Opacity" 0.5))

(fn `Path Material`
  (params (Tile :type "/Game/Blueprints/Tile_BP Object Reference"))
  (bind _gridmat_ref (`/Game/Blueprints/Tile_BP.GridMat_Ref` Tile))
  (`SceneComponent.SetVisibility` (`/Game/Blueprints/Tile_BP.Tile` Tile) true false)
  (`MaterialInstanceDynamic.SetVectorParameterValue` _gridmat_ref "BaseColor" (struct :`R` 0.479167 :`G` 0.392362 :`B` 0.104984 :`A` 1.0))
  (`MaterialInstanceDynamic.SetScalarParameterValue` _gridmat_ref "Opacity" 0.5))

(fn `Tracing Attackable Material`
  (params (Tile :type "/Game/Blueprints/Tile_BP Object Reference"))
  (bind _gridmat_ref (`/Game/Blueprints/Tile_BP.GridMat_Ref` Tile))
  (bind _returnvalue (`self.CheckPlayerController`))
  (if _returnvalue
    (`SceneComponent.SetVisibility` (`/Game/Blueprints/Tile_BP.Tile` Tile) true false)
    (`MaterialInstanceDynamic.SetVectorParameterValue` _gridmat_ref "BaseColor" (struct :`R` 0.401042 :`B` 0.026071 :`A` 1.0))
    (`MaterialInstanceDynamic.SetScalarParameterValue` _gridmat_ref "Opacity" 0.5)))

(fn `Tracing Material`
  (params (Tile :type "/Game/Blueprints/Tile_BP Object Reference"))
  (bind _gridmat_ref (`/Game/Blueprints/Tile_BP.GridMat_Ref` Tile))
  (`SceneComponent.SetVisibility` (`/Game/Blueprints/Tile_BP.Tile` Tile) true false)
  (`MaterialInstanceDynamic.SetVectorParameterValue` _gridmat_ref "BaseColor" (struct :`R` 0.692708 :`G` 0.678877 :`B` 0.125919 :`A` 1.0))
  (`MaterialInstanceDynamic.SetScalarParameterValue` _gridmat_ref "Opacity" 0.5))

(fn `Tracing Movable Material`
  (params (Tile :type "/Game/Blueprints/Tile_BP Object Reference"))
  (bind _gridmat_ref (`/Game/Blueprints/Tile_BP.GridMat_Ref` Tile))
  (bind _returnvalue (`self.CheckPlayerController`))
  (if _returnvalue
    (`SceneComponent.SetVisibility` (`/Game/Blueprints/Tile_BP.Tile` Tile) true false)
    (`MaterialInstanceDynamic.SetVectorParameterValue` _gridmat_ref "BaseColor" (struct :`R` 0.047614 :`G` 0.177083 :`B` 0.026365 :`A` 1.0))
    (`MaterialInstanceDynamic.SetScalarParameterValue` _gridmat_ref "Opacity" 0.5)))

(fn `UserConstructionScript`)