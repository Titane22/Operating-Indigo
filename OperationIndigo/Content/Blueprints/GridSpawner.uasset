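; Grid spawner actor that builds a GridX by GridY field of Tile_BP actors when play begins.
; A nested loop spawns tiles at GridSize spacing, offset by half the grid extent to lay them out around the spawner's location.
; Each tile joins GridArray, which is passed to OI_PlayerController_BP through InitGridArray after every spawn, rather than once when the grid completes.
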(event `self.ReceiveBeginPlay`
  (bind _gridsize (`self.GridSize`))
  (bind _gridx (`self.GridX`))
  (bind _gridy (`self.GridY`))
  (bind _gridsize_2 (`self.GridSize`))
  (bind _gridarray (`self.GridArray`))
  ;[1 1 1] Set Up Grid Scale
  (for _index (range 1 (+ _gridx 1))
    (for _index_2 (range 1 (+ _gridy 1))
      ;[1 1 1] Spawn Grid Add to Array
      (bind _returnvalue (`|SpawnActorFromClass` "/Game/Blueprints/Tile_BP.Tile_BP_C" (`KismetMathLibrary.MakeTransform` (+ (`KismetMathLibrary.MakeVector` (`KismetMathLibrary.Conv_IntToDouble` (- (* _index _gridsize_2) (/ (* _gridx _gridsize) 2))) (`KismetMathLibrary.Conv_IntToDouble` (- (* _index_2 _gridsize_2) (/ (* _gridy _gridsize) 2)))) (`self.K2_GetActorLocation`))) "AlwaysSpawn" "OverrideRootScale" null null))
      (`KismetArrayLibrary.Array_Add` _gridarray _returnvalue)
      (bind _asoi_player_controller_bp (cast `/Game/Blueprints/OI_PlayerController_BP` (`GameplayStatics.GetPlayerController` 0)))
      (`OperationIndigoPlayerController.InitGridArray` _asoi_player_controller_bp _gridarray))))

(fn `UserConstructionScript`)