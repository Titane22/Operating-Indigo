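; Tactical camera actor that the player moves, rotates and zooms.
; Forward and right axis inputs apply unswept local offsets scaled by move speed, without delta-time scaling.
; A Gate opened and closed by the rotate events passes mouse X into local yaw, so the camera turns only while rotation is active.
; Zoom inputs step the spring arm length within minimum and maximum limits.
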(event `InputAxis|MoveForward`
  (params (AxisValue :type "Float (single-precision)"))
  ;[1 1 1] Movement Forward and Right
  (`self.K2_AddActorLocalOffset` (`KismetMathLibrary.MakeVector` (* AxisValue (`self.MoveSpeed`)))))

(event `InputAxisKey|MouseX`
  (params (AxisValue :type "Float (single-precision)"))
  ;[1 1 1] Rotate Camera
  (`/Engine/EditorBlueprintResources/StandardMacros.Gate` true :!label _label
    (:`Exit`
      (`self.K2_AddActorLocalRotation` (`KismetMathLibrary.MakeRotator` 0.0 0.0 (* AxisValue (`self.RotateSpeed`)))))))

(event `InputAxis|MoveRight`
  (params (AxisValue :type "Float (single-precision)"))
  ;[1 1 1] Movement Forward and Right
  (`self.K2_AddActorLocalOffset` (`KismetMathLibrary.MakeVector` 0.0 (* AxisValue (`self.MoveSpeed`)))))

(event `self.RotateCamera`
  ;[1 1 1] Rotate Camera
  (goto _label :!via `Open`))

(event `self.RotateReleased`
  ;[1 1 1] Rotate Camera
  (goto _label :!via `Close`))

(event `InputAction|ZoomIn`
  (params (Key :type "Key Structure"))
  (bind _springarm (`self.SpringArm`))
  ;[1 1 1] Zoom In&Out
  (:`Pressed`
    (set `SpringArmComponent.TargetArmLength` (`KismetMathLibrary.FClamp` (- (`SpringArmComponent.TargetArmLength` _springarm) 50.0) (`self.MinArmLange`) (`self.MaxArmLange`)) _springarm)))

(event `InputAction|ZoomOut`
  (params (Key :type "Key Structure"))
  (bind _springarm (`self.SpringArm`))
  ;[1 1 1] Zoom In&Out
  (:`Pressed`
    (set `SpringArmComponent.TargetArmLength` (`KismetMathLibrary.FClamp` (- (`SpringArmComponent.TargetArmLength` _springarm) -50.0) (`self.MinArmLange`) (`self.MaxArmLange`)) _springarm)))

(fn `UserConstructionScript`)